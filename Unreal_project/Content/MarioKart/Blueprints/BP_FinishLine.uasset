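; Finish line trigger for the kart race that counts laps and ends the race.
; When an Unreal_projectPawn overlaps its Box with HitCheckpoint set, that pawn's LapsCompleted goes up by one.
; Reaching exactly three laps disables CanDrive on every such pawn in the level, stopping all racers.
; The node that would clear HitCheckpoint is unwired, so the flag is not reset here.
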(event `self.Box.OnComponentBeginOverlap`
  (params (OverlappedComponent :type "PrimitiveComponent Object Reference") (OtherActor :type "Actor Object Reference") (OtherComp :type "PrimitiveComponent Object Reference") (OtherBodyIndex :type Integer) (bFromSweep :type Boolean) (SweepResult :type "HitResult Structure (by ref)"))
  (bind _asunreal_project_pawn (cast `Unreal_projectPawn` OtherActor))
  (if (`Unreal_projectPawn.bHitCheckpoint` _asunreal_project_pawn)
    (bind _output_get (set `Unreal_projectPawn.LapsCompleted` (+ (`Unreal_projectPawn.LapsCompleted` _asunreal_project_pawn) 1) _asunreal_project_pawn))
    (if (== _output_get 3)
      (bind _outactors (`GameplayStatics.GetAllActorsOfClass` "/Script/Unreal_project.Unreal_projectPawn"))
      (for _array_element _outactors
        (set `Unreal_projectPawn.bCanDrive` false _array_element)))))

(fn `UserConstructionScript`)