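; BP_PowerUpBox is a Mario Kart-style item box pickup that increments the power-up count of an overlapping Unreal_projectPawn.
; Tick spins the cube on all axes and bobs it with a sine wave around the height cached at BeginPlay.
; On box overlap it plays a pickup sound, hides and disables collision, then respawns itself after a Delay.
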(event `self.ReceiveBeginPlay`
  (bind (_relativelocation_x _relativelocation_y _relativelocation_z) (`KismetMathLibrary.BreakVector` (`SceneComponent.RelativeLocation` (`self.Cube`))))
  (bind _output_get (set `self.Start Height` _relativelocation_z)))

(event `self.ReceiveTick`
  (params (DeltaSeconds :type "Float (single-precision)"))
  (`SceneComponent.K2_AddRelativeRotation` (`self.Cube`) (struct :`Pitch` 2.0 :`Yaw` 3.0 :`Roll` 1.0) false false)
  (`SceneComponent.K2_SetRelativeLocation` (`self.Cube`) (`KismetMathLibrary.MakeVector` 0.0 0.0 (+ (* (`KismetMathLibrary.Sin` (* (`GameplayStatics.GetTimeSeconds`) 1.0)) 15.0) (stale `self.ReceiveBeginPlay` _output_get))) false false))

(event `self.Box.OnComponentBeginOverlap`
  (params (OverlappedComponent :type "PrimitiveComponent Object Reference") (OtherActor :type "Actor Object Reference") (OtherComp :type "PrimitiveComponent Object Reference") (OtherBodyIndex :type Integer) (bFromSweep :type Boolean) (SweepResult :type "HitResult Structure (by ref)"))
  (bind _asunreal_project_pawn (cast `Unreal_projectPawn` OtherActor))
  (set `Unreal_projectPawn.PowerUpCount` (+ (`Unreal_projectPawn.PowerUpCount` _asunreal_project_pawn) 1) _asunreal_project_pawn)
  (`GameplayStatics.PlaySoundAtLocation` "/Game/Audio/Item_collect/Item_Cue.Item_Cue" (`self.K2_GetActorLocation`) (struct) 1.0 1.0 0.0 null null null null)
  (`self.SetActorHiddenInGame` true)
  (`self.SetActorEnableCollision` false)
  (`KismetSystemLibrary.Delay` 25.0)
  (`self.SetActorHiddenInGame` false)
  (`self.SetActorEnableCollision` true))

(fn `UserConstructionScript`)